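; BP_NPC is an interactable NPC that shows a sequence of dialogue lines to the player.
; On BeginPlay it creates a hidden WBP_Dialogue widget, and Interact shows it with the current entry from the Dialogues array.
; The widget's continue event advances the index, then hides the widget and resets to the first line after the last entry.
; Interaction queries and setters are forwarded to its InteractableComponent.
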(event `self.ReceiveBeginPlay`
  (bind _returnvalue (`|CreateWidget` "/Game/Blueprints/UI/Dialogue/WBP_Dialogue.WBP_Dialogue_C"))
  (bind _output_get (set `self.DialogueWidget` _returnvalue))
  (add `/Game/Blueprints/UI/Dialogue/WBP_Dialogue.DialogueContinued` _output_get (`|CreateDelegate` :!event `OnDialogueContinued`))
  (`UserWidget.AddToViewport` _output_get 0)
  (`/Game/Blueprints/UI/Dialogue/WBP_Dialogue.Show` _output_get false))

(event `/Game/Blueprints/Modules/Interaction/BI_Interactable.Interact`
  (params (Interactor :type "Actor Object Reference") (InteractionAction :type "InputAction Object Reference"))
  (bind _dialoguewidget (`self.DialogueWidget`))
  (`/Game/Blueprints/UI/Dialogue/WBP_Dialogue.SetText` _dialoguewidget (`self.GetCurrentDialogueText`))
  (`/Game/Blueprints/UI/Dialogue/WBP_Dialogue.Show` _dialoguewidget true))

(fn `GetCurrentDialogueText`
  (returns (Text :type "Text (by ref)"))
  (return (`|GetArrayItem` (`self.Dialogues`) (`self.DialogueIndex`))))

(fn `GetInteractionMethod`
  (returns (Method :type "/Game/Blueprints/Modules/Interaction/BI_InteractionMethod Interface"))
  (bind _method (`/Game/Blueprints/Modules/Interaction/AC_InteractableComponent.GetInteractionMethod` (`self.InteractableComponent`)))
  (return _method))

(fn `IsActionInteractable`
  (params (Action :type "InputAction Object Reference"))
  (returns (IsInteractable :type Boolean))
  (bind _isinteractable (`/Game/Blueprints/Modules/Interaction/AC_InteractableComponent.IsActionInteractable` (`self.InteractableComponent`) Action))
  (return _isinteractable))

(fn `IsInteractable`
  (returns (Interactable :type Boolean))
  (bind _interactable (`/Game/Blueprints/Modules/Interaction/AC_InteractableComponent.IsInteractable` (`self.InteractableComponent`)))
  (return _interactable))

(fn `OnDialogueContinued`
  (bind _result (`/Engine/EditorBlueprintResources/StandardMacros.IncrementInt` (`self.DialogueIndex`))
    (:`  `
      (if (< _result (`KismetArrayLibrary.Array_Length` (`self.Dialogues`)))
        (`/Game/Blueprints/UI/Dialogue/WBP_Dialogue.SetText` (`self.DialogueWidget`) (`self.GetCurrentDialogueText`))
        (else
          (set `self.DialogueIndex` 0)
          (`/Game/Blueprints/UI/Dialogue/WBP_Dialogue.Show` (`self.DialogueWidget`) false))))))

(fn `SetInteractable`
  (params (Interactable :type Boolean))
  (returns (CurrentInteractable :type Boolean))
  (bind _currentinteractable (`/Game/Blueprints/Modules/Interaction/AC_InteractableComponent.SetInteractable` (`self.InteractableComponent`) Interactable))
  (return _currentinteractable))

(fn `UserConstructionScript`)