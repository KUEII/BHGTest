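; BP_CollectableItem is a world pickup actor that passes its item ID to whoever interacts with it, then destroys itself.
; The construction script looks up the ID in DT_ItemData, sets the row's mesh and scales it by bounding-sphere radius so items share a unified size.
; Interactability queries and the setter are forwarded to its InteractableComponent.
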(event `/Game/Blueprints/Modules/Interaction/BI_Interactable.Interact`
  (params (Interactor :type "Actor Object Reference") (InteractionAction :type "InputAction Object Reference"))
  (message `/Game/Blueprints/Inventory/BI_InventoryOwner.CollectItem` Interactor (`self.ItemID`) 0)
  (`self.K2_DestroyActor`))

(fn `GetInteractionMethod`
  (returns (Method :type "/Game/Blueprints/Modules/Interaction/BI_InteractionMethod Interface"))
  (bind _method (`/Game/Blueprints/Modules/Interaction/AC_InteractableComponent.GetInteractionMethod` (`self.InteractableComponent`)))
  (return _method))

(fn `IsActionInteractable`
  (params (Action :type "InputAction Object Reference"))
  (returns (IsInteractable :type Boolean))
  (bind _isinteractable (`/Game/Blueprints/Modules/Interaction/AC_InteractableComponent.IsActionInteractable` (`self.InteractableComponent`) Action))
  (return _isinteractable))

(fn `IsInteractable`
  (returns (Interactable :type Boolean))
  (bind _interactable (`/Game/Blueprints/Modules/Interaction/AC_InteractableComponent.IsInteractable` (`self.InteractableComponent`)))
  (return _interactable))

(fn `SetInteractable`
  (params (Interactable :type Boolean))
  (returns (CurrentInteractable :type Boolean))
  (bind _currentinteractable (`/Game/Blueprints/Modules/Interaction/AC_InteractableComponent.SetInteractable` (`self.InteractableComponent`) Interactable))
  (return _currentinteractable))

(fn `UserConstructionScript`
  (bind _staticmesh (`self.StaticMesh`))
  (bind _returnvalue (`|GetDataTableRow` "/Game/Blueprints/Inventory/Item/DT_ItemData.DT_ItemData" (`.RowName` (break `DataTableRowHandle` (`self.ItemID`))))
    (:`then`
      (`StaticMeshComponent.SetStaticMesh` _staticmesh (`.Mesh_8_A117DF2946896789A305AFB34DF08364` (break `/Game/Blueprints/Inventory/Item/F_ItemData` _returnvalue)))
      (bind (_returnvalue_origin _returnvalue_boxextent _returnvalue_sphereradius) (`KismetMathLibrary.BreakBoxSphereBounds` (`StaticMesh.GetBounds` (`.Mesh_8_A117DF2946896789A305AFB34DF08364` (break `/Game/Blueprints/Inventory/Item/F_ItemData` _returnvalue)))))
      (`SceneComponent.SetRelativeScale3D` _staticmesh (`KismetMathLibrary.Conv_DoubleToVector` (/ (`self.UnifiedRadius`) _returnvalue_sphereradius))))))