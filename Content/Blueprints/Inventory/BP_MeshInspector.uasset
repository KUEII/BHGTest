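; Inventory mesh inspector actor that shows a single static mesh to a scene capture camera restricted to this actor's components.
; SetMesh resets the camera and scales each new mesh by its bounding sphere to a unified radius, so different meshes frame alike.
; Cursor deltas orbit the camera through accumulated yaw and clamped pitch, re-aiming it at the actor.
; Zoom is clamped and divides the base camera distance along the current view direction.
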(fn `AddPitchYaw`
  (params (Delta :type "Vector2D Structure"))
  (returns (ClampedDelta :type "Vector2D Structure") (Pitch :type "Float (double-precision)") (Yaw :type "Float (double-precision)"))
  (locals (LastPitch :type "Float (double-precision)" :default 0.0) (LastYaw :type "Float (double-precision)" :default 0.0))
  (bind (_delta_x _delta_y) (`KismetMathLibrary.BreakVector2D` (`local.Delta`)))
  (bind _maxpitch (`self.MaxPitch`))
  (bind _yaw (`self.Yaw`))
  (set `local.LastYaw` _yaw)
  (set `local.LastPitch` (`self.Pitch`))
  (bind _output_get (set `self.Yaw` (+ _yaw _delta_x)))
  (bind _output_get_2 (set `self.Pitch` (`KismetMathLibrary.ClampAngle` (+ _delta_y (`self.Pitch`)) (* _maxpitch -1.0) _maxpitch)))
  (return (`KismetMathLibrary.MakeVector2D` (- _output_get (`local.LastYaw`)) (- _output_get_2 (`local.LastPitch`))) (`self.Pitch`) (`self.Yaw`)))

(fn `HasMesh`
  (returns (Has :type Boolean))
  (return (`KismetSystemLibrary.IsValid` (`StaticMeshComponent.StaticMesh` (`self.StaticMesh`)))))

(fn `ResetCamera`
  (bind _scenecapturecomponent2d (`self.SceneCaptureComponent2D`))
  (`SceneComponent.K2_SetRelativeRotation` _scenecapturecomponent2d (struct :`Yaw` 180.0) false false)
  (`SceneComponent.K2_SetRelativeLocation` _scenecapturecomponent2d (`KismetMathLibrary.MakeVector` (`self.CameraDistance`)) false true)
  (set `self.Zoom` 1.0)
  (set `self.Pitch` 0.0)
  (set `self.Yaw` 0.0))

(fn `RotateCameraByCursor`
  (params (Delta :type "Vector2D Structure"))
  (bind (_clampeddelta _pitch _yaw) (`self.AddPitchYaw` Delta))
  (`self.RotateToPitchYaw` _pitch _yaw))

(fn `RotateToPitchYaw`
  (params (Pitch :type "Float (double-precision)") (Yaw :type "Float (double-precision)"))
  (bind _scenecapturecomponent2d (`self.SceneCaptureComponent2D`))
  (`SceneComponent.K2_SetRelativeLocation` (`self.SceneCaptureComponent2D`) (* (`KismetMathLibrary.Normal` (`KismetMathLibrary.GreaterGreater_VectorRotator` (`KismetMathLibrary.Vector_Forward`) (`KismetMathLibrary.MakeRotator` 0.0 Pitch Yaw))) (/ (`self.CameraDistance`) (`self.Zoom`))) false true)
  (`SceneComponent.K2_SetWorldRotation` _scenecapturecomponent2d (`KismetMathLibrary.FindLookAtRotation` (`SceneComponent.K2_GetComponentLocation` _scenecapturecomponent2d) (`self.K2_GetActorLocation`)) false false))

(fn `SetMesh`
  (params (NewMesh :type "StaticMesh Object Reference"))
  (bind (_returnvalue_origin _returnvalue_boxextent _returnvalue_sphereradius) (`KismetMathLibrary.BreakBoxSphereBounds` (`StaticMesh.GetBounds` NewMesh)))
  (bind _staticmesh (`self.StaticMesh`))
  (`self.ResetCamera`)
  (`SceneComponent.SetRelativeScale3D` _staticmesh (`KismetMathLibrary.Conv_DoubleToVector` (/ (`self.UnifiedRadius`) _returnvalue_sphereradius)))
  (`StaticMeshComponent.SetStaticMesh` _staticmesh (`local.NewMesh`)))

(fn `UserConstructionScript`
  (`SceneCaptureComponent.ShowOnlyActorComponents` (`self.SceneCaptureComponent2D`) self false)
  (`SceneComponent.K2_SetRelativeLocation` (`self.SceneCaptureComponent2D`) (`KismetMathLibrary.MakeVector` (`self.CameraDistance`)) false true))

(fn `ZoomIn`
  (params (Delta :type "Float (double-precision)"))
  (bind _scenecapturecomponent2d (`self.SceneCaptureComponent2D`))
  (bind _output_get (set `self.Zoom` (`KismetMathLibrary.FClamp` (+ (* Delta (`self.ZoomSensitivity`)) (`self.Zoom`)) 0.5 2.0)))
  (`SceneComponent.K2_SetRelativeLocation` _scenecapturecomponent2d (* (`KismetMathLibrary.Normal` (`SceneComponent.RelativeLocation` _scenecapturecomponent2d)) (/ (`self.CameraDistance`) _output_get)) false true))