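; Inventory component that holds a fixed-size array of item slots and owns the inventory UI widget.
; On BeginPlay it sizes the slots and creates the widget collapsed, passing itself in, and IA_Inventory toggles its visibility.
; AddItem fills the first empty slot if the ID exists in DT_ItemData, and ChangeSlot swaps two slots.
; Both broadcast InventoryUpdated after changing the array.
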(event `self.ReceiveBeginPlay`
  (`KismetArrayLibrary.Array_Resize` (`self.Slots`) (`self.Size`))
  (bind _returnvalue (`|CreateWidget` "/Game/Blueprints/UI/Inventory/WBP_Inventory.WBP_Inventory_C" null self))
  (bind _output_get (set `self.InventoryUI` _returnvalue))
  (`UserWidget.AddToViewport` _output_get 0)
  (`Widget.SetVisibility` (`self.InventoryUI`) "Collapsed"))

(event `EnhancedInput|/Game/Assets/Inputs/IA_Inventory`
  (params (ActionValue :type Boolean) (ElapsedSeconds :type "Float (double-precision)") (TriggeredSeconds :type "Float (double-precision)") (InputAction :type "InputAction Object Reference" :default "/Game/Assets/Inputs/IA_Inventory.IA_Inventory"))
  (bind _inventoryui (`self.InventoryUI`))
  (:`Triggered`
    (`/Game/Blueprints/UI/Inventory/WBP_Inventory.Show` _inventoryui (not (`Widget.IsVisible` _inventoryui)))))

(fn `AddItem`
  (params (ID :type "DataTableRowHandle Structure (by ref)"))
  (locals (EmptySlot :type Integer :default 0))
  (bind _output_get (set `local.EmptySlot` (`self.FindEmptySlot`)))
  (if (>= _output_get 0)
    (`|GetDataTableRow` "/Game/Blueprints/Inventory/Item/DT_ItemData.DT_ItemData" (`.RowName` (break `DataTableRowHandle` (`local.ID`)))
      (:`then`
        (`KismetArrayLibrary.Array_Set` (`self.Slots`) (`local.EmptySlot`) (make `/Game/Blueprints/Inventory/F_InventorySlot` (`local.ID`)))
        (`self.InventoryUpdated`)))))

(fn `ChangeSlot`
  (params (Index1 :type Integer) (Index2 :type Integer))
  (locals (TempSlot :type "/Game/Blueprints/Inventory/F_InventorySlot Structure"))
  (bind _slots (`self.Slots`))
  (set `local.TempSlot` (`|GetArrayItem` (`self.Slots`) Index1))
  (`KismetArrayLibrary.Array_Set` _slots (`local.Index1`) (`|GetArrayItem` (`self.Slots`) Index2))
  (`KismetArrayLibrary.Array_Set` _slots (`local.Index2`) (`local.TempSlot`))
  (`self.InventoryUpdated`))

(fn `FindEmptySlot`
  (returns (Index :type Integer))
  (for (_array_element _array_index) (`self.Slots`)
    (bind (_itemid_datatable _itemid_rowname) (break `DataTableRowHandle` (break `/Game/Blueprints/Inventory/F_InventorySlot` _array_element)))
    (if (== _itemid_rowname "None")
      (return _array_index)))
  (return -1))

(fn `GetSlots`
  (returns (Slots :type "Array of /Game/Blueprints/Inventory/F_InventorySlot Structure"))
  (return (`self.Slots`)))

(fn `Print`
  (for _array_element (`self.Slots`)
    (bind (_itemid_datatable _itemid_rowname) (break `DataTableRowHandle` (break `/Game/Blueprints/Inventory/F_InventorySlot` _array_element)))
    (`KismetSystemLibrary.PrintString` (`KismetStringLibrary.Conv_NameToString` _itemid_rowname))))