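; Actor component that detects the interactable actor in front of its owner's camera and tracks it as the current target.
; A Delay on Tick throttles line traces cast from the camera location along its forward vector, keeping hits that report as interactable through interface messages.
; Target changes toggle listener state on the old and new actors and raise detected, changed or undetected notifications.
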(event `self.ReceiveBeginPlay`
  (set `self.Interactor` (`self.GetOwner`)))

(event `self.ReceiveTick`
  (params (DeltaSeconds :type "Float (single-precision)"))
  (`KismetSystemLibrary.Delay` (`self.CastInterval`))
  (`self.Cast`))

(event `Cast`
  (bind _interactor (`self.Interactor`))
  (bind _forward (message `/Game/Blueprints/Interfaces/BI_CameraInfoProvider.GetCameraForward` _interactor))
  (bind _location (message `/Game/Blueprints/Interfaces/BI_CameraInfoProvider.GetCameraLocation` _interactor))
  (bind _interactableobject (`self.Raycast` _location _forward))
  (`self.SetInteractableTarget` _interactableobject))

(fn `GetTarget`
  (returns (Target :type "Actor Object Reference"))
  (return (`self.InteractableTarget`)))

(fn `Raycast`
  (params (StartLocation :type "Vector Structure") (Direction :type "Vector Structure"))
  (returns (InteractableObject :type "Actor Object Reference"))
  (bind (_startpoint _endpoint) (`/Game/Blueprints/Utilities/BPFL_Trace.GetTraceEndPoints` StartLocation Direction (`self.CastRange`)))
  (bind (_outhit _returnvalue) (`KismetSystemLibrary.LineTraceSingle` :`Start` _startpoint :`End` _endpoint :`TraceChannel` (`self.TraceChannel`) :`DrawDebugType` (select `bool` (`self.DebugTrace`) :`true` "ForDuration" :!type "EDrawDebugTrace Enum")))
  (bind (_bblockinghit _binitialoverlap _time _distance _location _impactpoint _normal _impactnormal _physmat _hitactor) (`GameplayStatics.BreakHitResult` _outhit))
  (bind _interactable (message `/Game/Blueprints/Modules/Interaction/BI_Interactable.IsInteractable` _hitactor))
  (if (and _interactable _returnvalue)
    (return _hitactor)
    (else
      (return null))))

(fn `SetInteractableTarget`
  (params (Target :type "Actor Object Reference"))
  (locals (OldTarget :type "Actor Object Reference"))
  (bind _oldtarget (`local.OldTarget`))
  (if (!= (`self.InteractableTarget`) Target)
    (bind _interactabletarget (`self.InteractableTarget`)
      (:`then`
        (bind _output_get (set `local.OldTarget` _interactabletarget))
        (message `/Game/Blueprints/Modules/Interaction/BI_Interactable.SetAsListener` _output_get false)
        (bind _output_get_2 (set `self.InteractableTarget` (`local.Target`)))
        (`/Engine/EditorBlueprintResources/StandardMacros.IsValid` _output_get_2
          (:`Is Valid`
            (message `/Game/Blueprints/Modules/Interaction/BI_Interactable.SetAsListener` _output_get_2 true)
            (`self.InteractableChanged` _oldtarget _output_get_2))
          (:`Is Not Valid`
            (`self.InteractableUndetected` _oldtarget))))
      (:`else`
        (bind _output_get_3 (set `self.InteractableTarget` Target))
        (message `/Game/Blueprints/Modules/Interaction/BI_Interactable.SetAsListener` _output_get_3 true)
        (`self.InteractableDetected` _output_get_3)))))