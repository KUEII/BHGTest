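; AC_InteractableComponent is an actor component that marks its owner as interactable and exposes how it can be interacted with.
; It holds an InteractionMethod object and an Interactable flag with getter and setter functions.
; IsActionInteractable checks whether a given input action is used by any prompt in the method's interaction prompt list, without consulting the flag.
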(fn `GetInteractionMethod`
  (returns (Method :type "/Game/Blueprints/Modules/Interaction/BI_InteractionMethod Interface"))
  (return (`self.InteractionMethod`)))

(fn `IsActionInteractable`
  (params (Action :type "InputAction Object Reference"))
  (returns (IsInteractable :type Boolean))
  (bind _newparam (`/Game/Blueprints/Modules/Interaction/BI_InteractionMethod.GetInteractionPromptList` (`self.InteractionMethod`)))
  (for _array_element _newparam
    (bind _usinginputaction (`/Game/Blueprints/Modules/Interaction/BI_InteractionPrompt.IsUsingInputAction` _array_element Action))
    (if _usinginputaction
      (return true)))
  (return false))

(fn `IsInteractable`
  (returns (Interactable :type Boolean))
  (return (`self.Interactable`)))

(fn `SetInteractable`
  (params (Interactable :type Boolean))
  (returns (CurrentInteractable :type Boolean))
  (bind _output_get (set `self.Interactable` Interactable))
  (return _output_get))